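; BP_Gaz is a gas particle actor that represents oxygen, polluted oxygen, carbon dioxide or hydrogen as a colored cube.
; The construction script uses EGazType to set material, breathability, condensation point, temperature and density, deriving pressure as temperature over density.
; BeginPlay starts two fast looping timers, alongside custom events for debug printing and interpolated movement with no target wired.
; Molecule state, condensation and opacity logic is present but disconnected.
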(event Custom|Custom_Tick
  (Development|PrintString (Utilities|String|ToString(Text) (Utilities|Text|FormatText "Gaz_Type : {A} 
Temperature : {B} 
Density : {C} 
Breathable_? : {D}" (Utilities|String|EnumtoString (Variables|Default|GetE_Gaz_Type)) (Variables|Default|GetTemperature) (Variables|Default|GetDensity) (Variables|Default|GetBreathable_?))) true true "(R=1.000000,G=0.000000,B=0.000000,A=1.000000)" 0.09))

(event Custom|Particle_Movement
  (Transformation|SetActorLocation (Math|Interpolation|VInterpTo (Transformation|GetWorldLocation (Variables|Default|GetCube)) "0, 0, 0" 1.0 0.2) false false))

(event EventBeginPlay
  (Utilities|Time|SetTimerbyEvent (EventDispatchers|CreateEvent :!event Custom|Custom_Tick) 0.09 true)
  (Variables|Default|SetMolecule_State (Math|Integer|Clamp(Integer) (Variables|Default|GetMolecule_State) 0 2))
  (Utilities|Time|SetTimerbyEvent (EventDispatchers|CreateEvent :!event Custom|Particle_Movement) 0.09 true))

(event EventTick
  (params (DeltaSeconds :type Float%20%28single-precision%29)))

(fn ConstructionScript
  (switch Utilities|FlowControl|Switch|SwitchonE_Gaz_Type (Variables|Default|GetE_Gaz_Type)
    (:NewEnumerator0
      (Rendering|Material|SetMaterial (Variables|Default|GetCube) 0 "/Game/Gaz/Material/MI_Oxygen_Color.MI_Oxygen_Color")
      (Variables|Default|SetBreathable_? true)
      (Variables|Default|SetCondensation_Point -182.96)
      (Variables|Default|SetTemperature 22.0)
      (Variables|Default|SetDensity 15.9994)
      (Variables|Default|SetPressure (/ (Variables|Default|GetTemperature) (Variables|Default|GetDensity))))
    (:NewEnumerator1
      (Rendering|Material|SetMaterial (Variables|Default|GetCube) 0 "/Game/Gaz/Material/MI_Polluted_Oxygen_Color.MI_Polluted_Oxygen_Color")
      (Variables|Default|SetBreathable_? true)
      (Variables|Default|SetCondensation_Point -182.96)
      (Variables|Default|SetTemperature 22.0)
      (Variables|Default|SetDensity 15.9994)
      (Variables|Default|SetPressure (/ (Variables|Default|GetTemperature) (Variables|Default|GetDensity))))
    (:NewEnumerator2
      (Rendering|Material|SetMaterial (Variables|Default|GetCube) 0 "/Game/Gaz/Material/MI_Carbon_Dioxyde_Color.MI_Carbon_Dioxyde_Color")
      (Variables|Default|SetBreathable_? false)
      (Variables|Default|SetCondensation_Point -48.15)
      (Variables|Default|SetTemperature 27.0)
      (Variables|Default|SetDensity 44.01)
      (Variables|Default|SetPressure (/ (Variables|Default|GetTemperature) (Variables|Default|GetDensity))))
    (:NewEnumerator3
      (Rendering|Material|SetMaterial (Variables|Default|GetCube) 0 "/Game/Gaz/Material/MI_Hydrogen_Color.MI_Hydrogen_Color")
      (Variables|Default|SetBreathable_? false)
      (Variables|Default|SetCondensation_Point -252.15)
      (Variables|Default|SetTemperature 3e+01)
      (Variables|Default|SetDensity 1.00794)
      (Variables|Default|SetPressure (/ (Variables|Default|GetTemperature) (Variables|Default|GetDensity))))))