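; BP_Gaz_Spawner is an actor meant to spawn a capped number of randomly typed BP_Gaz actors at its SpawnPoint.
; BeginPlay resets the count and starts a looping timer at a random one-to-two-second interval, chosen once.
; The logic that spawns, assigns a random EGazType and clears the timer at NbrGazMax is disconnected.
; The Spawn event is empty, so no gaz spawns as wired.
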(event Custom|Spawn)

(event EventBeginPlay
  (Variables|Default|SetNbr_Of_Gaz 0)
  (bind _returnvalue (Utilities|Time|SetTimerbyEvent (EventDispatchers|CreateEvent :!event Custom|Spawn) (Math|Random|RandomFloatinRange 1.0 2.0) true))
  (Variables|Default|SetSpawn_Event_Ref _returnvalue))

(fn ConstructionScript)